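; BP_ClothoPlayerController is the Clotho player controller Blueprint that shows a player's finishing rank in a popup.
; BlueprintShowRankUI creates a UMG_Message widget, fills it with the rank as Chinese "Nth place" text plus a confirm button, and adds it to the viewport.
; The button's click is bound to RemoveSelf, which removes the popup.
; BeginPlay, Tick and the construction script are empty.
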(event Custom|RemoveSelf
  (Widget|RemovefromParent (stale EventBlueprintShowRankUI _returnvalue)))

(event EventBeginPlay)

(event EventTick
  (params (DeltaSeconds :type Float%20%28single-precision%29)))

(event EventBlueprintShowRankUI
  (params (Rank :type Integer))
  (bind _returnvalue (UserInterface|CreateWidget "/Game/Clotho/UI/Entry/UMG_Message.UMG_Message_C" self))
  (EventDispatchers|BindEventtoOnClicked (Variables|/Script/Clotho.MessageWidget|GetButton_One _returnvalue) (delegate Custom|RemoveSelf))
  (Variables|/Script/Clotho.MessageWidget|SetMessageText _returnvalue (Utilities|Text|FormatText "第{0}名" Rank))
  (Variables|/Script/Clotho.MessageWidget|SetButtonText _returnvalue "确定")
  (Variables|/Script/Clotho.MessageWidget|SetHasButton _returnvalue true)
  (UserInterface|Viewport|AddtoViewport _returnvalue 0))

(fn ConstructionScript)
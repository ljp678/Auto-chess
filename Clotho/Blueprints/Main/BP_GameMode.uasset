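; Game mode for Clotho that gives each joining player their own BP_Dragon at a numbered spawn point.
; PostLogin derives a zero-based index from the player count, finds the PlayerStart whose tag matches it, then spawns, indexes and possesses the dragon there.
; An empty SpawnDefaultPawnAtTransform override leaves pawn creation to that event.
; CheckPlayerNum reports whether the latest index fits within four players, though nothing here calls it.
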(event EventBeginPlay)

(event EventTick
  (params (DeltaSeconds :type Float%20%28single-precision%29)))

(event EventPostLogin
  (params (NewPlayer :type Player%20Controller%20Object%20Reference))
  (Variables|Default|SetPlayerCount_0 (- (Variables|Default|GetNumPlayers) 1))
  (bind _outactors (Actor|GetAllActorsOfClass "/Script/Engine.PlayerStart"))
  (bind _array_element (Utilities|Array|ForEachLoopwithBreak _outactors :!label _label)
    (:LoopBody
      (if (Utilities|Name|Equal(Name) (Variables|/Script/Engine.PlayerStart|GetPlayerStartTag _array_element) (Utilities|String|StringToName (Utilities|String|ToString(Integer) (Variables|Default|GetPlayerCount_0))))
        (Utilities|FlowControl|Sequence
          (:then_0
            (goto _label Break))
          (:then_1
            (bind _returnvalue (Game|SpawnActorfromClass "/Game/Clotho/Dragon/BP_Dragon.BP_Dragon_C" (Math|Transform|MakeTransform (Transformation|GetActorLocation _array_element) "0, 0, 0" "1,1,1") "Undefined" 0 0))
            (Variables|/Script/Clotho.DragonCharacter|SetPlayerIndex _returnvalue (Variables|Default|GetPlayerCount_0))
            (Pawn|Possess NewPlayer _returnvalue)))))))

(fn ConstructionScript)

(fn SpawnDefaultPawnatTransform
  (params (NewPlayer :type Controller%20Object%20Reference) (SpawnTransform :type Transform%20%28by%20ref%29))
  (return 0))

(fn CheckPlayerNum
  (params (PlayerController :type Player%20Controller%20Object%20Reference))
  (return (not (> (Variables|Default|GetPlayerCount_0) 3))))
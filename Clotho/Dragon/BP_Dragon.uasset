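; BP_Dragon is the dragon actor, which can be repositioned to tagged Player Start points in the level.
; SetDragonLocationbyIndex keeps the target player index if it matches the dragon's PlayerIndex, otherwise offsets it by four.
; It then searches all Player Starts for a tag equal to that number and moves the dragon to the first match.
; BeginPlay, overlap, Tick and construction logic are empty.
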(event EventBeginPlay)

(event Collision|EventActorBeginOverlap
  (params (OtherActor :type Actor%20Object%20Reference)))

(event EventTick
  (params (DeltaSeconds :type Float%20%28single-precision%29)))

(event EventSetDragonLocationbyIndex
  (params (TargetPlayerIndex :type Integer))
  (if (== TargetPlayerIndex (Variables|Default|GetPlayerIndex))
    (Variables|Default|SetTargetIndex TargetPlayerIndex)
    (else
      (Variables|Default|SetTargetIndex (+ TargetPlayerIndex 4))))
  (bind _outactors (Actor|GetAllActorsOfClass "/Script/Engine.PlayerStart"))
  (bind _array_element (Utilities|Array|ForEachLoopwithBreak _outactors :!label _label)
    (:LoopBody
      (if (Utilities|Name|Equal(Name) (Variables|/Script/Engine.PlayerStart|GetPlayerStartTag _array_element) (Utilities|String|StringToName (Utilities|String|ToString(Integer) (Variables|Default|GetTargetIndex))))
        (Utilities|FlowControl|Sequence
          (:then_0
            (goto _label Break))
          (:then_1
            (Transformation|SetActorLocation (Transformation|GetActorLocation _array_element) false false)))))))

(fn ConstructionScript)
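; PC_Entry is the entry-screen player controller that creates the remastered entry menu for the local player on BeginPlay.
; If its Text variable is non-empty, it shows a message popup with a confirm button that removes it, then immediately switches the entry menu.
; The Space action feeds the same DoOnce, so the menu switch fires only once from either path.
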(event Custom|ShowOptionMessage
  (if (not (Utilities|Text|TextIsEmpty (Variables|Default|GetText)))
    (Utilities|FlowControl|Sequence
      (:then_0
        (bind _returnvalue (UserInterface|CreateWidget "/Game/Clotho/UI/Entry/UMG_Message.UMG_Message_C" self))
        (EventDispatchers|BindEventtoOnClicked (Variables|/Script/Clotho.MessageWidget|GetButton_One _returnvalue) (delegate Custom|RemoveSelf))
        (Variables|/Script/Clotho.MessageWidget|SetMessageText _returnvalue (Variables|Default|GetText))
        (Variables|/Script/Clotho.MessageWidget|SetButtonText _returnvalue "确定")
        (Variables|/Script/Clotho.MessageWidget|SetHasButton _returnvalue true)
        (UserInterface|Viewport|AddtoViewport _returnvalue 0))
      (:then_1
        (Utilities|FlowControl|DoOnce false
          (:Completed
            (Default|SwitchMenu (Variables|Default|GetEntry%20Menu))))))))

(event Custom|RemoveSelf
  (Widget|RemovefromParent (stale Custom|ShowOptionMessage _returnvalue)))

(event EventBeginPlay
  (if (Pawn|IsLocalController)
    (bind _returnvalue (UserInterface|CreateWidget "/Game/Clotho/UI/Entry/UMG_EntryMenu_Remastered.UMG_EntryMenu_Remastered_C"))
    (bind _output_get (Variables|Default|SetEntry%20Menu _returnvalue))
    (UserInterface|Viewport|AddtoViewport _output_get 0)
    (CallFunction|ShowOptionMessage)))

(event EventTick
  (params (DeltaSeconds :type Float%20%28single-precision%29)))

(event Input|ActionEvents|InputActionSpace
  (params (Key :type Key%20Structure :default "None"))
  (:Pressed
    (Utilities|FlowControl|DoOnce false
      (:Completed
        (Default|SwitchMenu (Variables|Default|GetEntry%20Menu))))))

(fn ConstructionScript)